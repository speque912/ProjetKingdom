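; BP_LightningStrike is a short-lived lightning flash actor for the dynamic sky system.
; Play sets shadow casting on its Lightning light, scales MaxIntensity by the given intensity and starts the timeline.
; The Animate timeline runs at a randomized play rate, driving light intensity up to that maximum, and the actor destroys itself when it finishes.
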(event Custom|Timeline
  (Components|Timeline|SetPlayRate (Variables|Default|GetAnimate) (Math|Random|RandomFloatinRange 0.7 1.1))
  (bind _intensity (Timeline|Animate PlayFromStart)
    (:Update
      (Rendering|Components|Light|SetIntensity (Variables|Default|GetLightning) (Math|Float|Lerp 0.0 (Variables|Default|GetMax%20intensity) _intensity)))
    (:Finished
      (Actor|DestroyActor))))

(fn ConstructionScript)

(fn Play
  (params (shadow :type Boolean) (intensity :type Float%20%28single-precision%29))
  (Variables|Default|SetMax%20intensity (* intensity (Variables|Default|GetMax%20intensity)))
  (Rendering|Components|Light|SetCastShadows (Variables|Default|GetLightning) shadow)
  (CallFunction|Timeline))